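; Turret projectile that damages a combat character on contact and then destroys itself.
; On spawn its Box ignores the owner and all existing turret projectiles when moving, and a short lifespan is set.
; The Box's begin-overlap event applies the damage; other actors do not destroy it.
; A delayed timer enables an overlap-check flag that only disconnected leftover polling logic reads.
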(event `self.Box.OnComponentBeginOverlap`
  (params (OverlappedComponent :type "PrimitiveComponent Object Reference") (OtherActor :type "Actor Object Reference") (OtherComp :type "PrimitiveComponent Object Reference") (OtherBodyIndex :type Integer) (bFromSweep :type Boolean) (SweepResult :type "HitResult Structure (by ref)"))
  (bind _asbp_combat_character (cast `/Game/Variant_Combat/Blueprints/BP_CombatCharacter` OtherActor))
  (`GameplayStatics.ApplyDamage` _asbp_combat_character 0.5)
  (`self.K2_DestroyActor`))

(event `self.ReceiveBeginPlay`
  (`PrimitiveComponent.IgnoreActorWhenMoving` (`self.Box`) (`self.GetOwner`) true)
  (bind _outactors (`GameplayStatics.GetAllActorsOfClass` "BP_TurretProjectile_C"))
  (for _array_element _outactors
    (`PrimitiveComponent.IgnoreActorWhenMoving` (`self.Box`) _array_element true)
    (`KismetSystemLibrary.K2_SetTimer` null "EnableOverlapCheck" 0.2))
  (`self.SetLifeSpan` 1.0))

(event `self.ReceiveTick`
  (params (DeltaSeconds :type "Float (single-precision)")))

(event `EnableOverlapCheck`
  (set `self.IsCheckingOverlaps` true))

(fn `UserConstructionScript`)