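; BP_Turret is a turret that spins continuously while firing a steady stream of projectiles.
; Tick yaws the whole actor by RotationSpeed scaled with delta time, with no targeting logic.
; A fast looping timer started on BeginPlay calls FireProjectile, which spawns a BP_TurretProjectile at the MuzzleDirection component's transform and sets the turret as its owner.
; A single ApplyDamage call destroys the turret, as it tracks no health.
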(event `self.ReceiveBeginPlay`
  (`KismetSystemLibrary.K2_SetTimer` null "FireProjectile" 0.1 true))

(event `self.ReceiveTick`
  (params (DeltaSeconds :type "Float (single-precision)"))
  (`self.K2_AddActorLocalRotation` (`KismetMathLibrary.MakeRotator` 0.0 0.0 (* DeltaSeconds (`self.RotationSpeed`)))))

(event `/Game/Variant_Combat/Blueprints/BPI_Damageable.Apply Damage`
  (params (Damage :type "Float (double-precision)") (`Damage Causer` :type "Actor Object Reference") (`Damage Location` :type "Vector Structure") (`Damage Impulse` :type "Vector Structure"))
  (`self.K2_DestroyActor`))

(fn `FireProjectile`
  (bind _returnvalue (`|SpawnActorFromClass` "/Game/ProjectSkyjet/Blueprints/BP_TurretProjectile.BP_TurretProjectile_C" (`KismetMathLibrary.MakeTransform` (`SceneComponent.K2_GetComponentLocation` (`self.MuzzleDirection`)) (`SceneComponent.K2_GetComponentRotation` (`self.MuzzleDirection`))) "AlwaysSpawn" "MultiplyWithRoot" null null))
  (`self.SetOwner` _returnvalue self))

(fn `UserConstructionScript`)