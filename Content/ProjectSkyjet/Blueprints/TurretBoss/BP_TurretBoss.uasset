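; BP_TurretBoss is a turret boss that fires missiles at the player when within range and completes the level when destroyed.
; Tick checks player distance and calls FireMissile, which spawns an AGM114 missile from one of two arrows at random, with a short timer resetting the CanFire cooldown.
; Its ApplyDamage event subtracts Health and, only when it equals exactly zero, calls HandleDeath to destroy the actor and show WB_LevelComplete.
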(event `self.ReceiveBeginPlay`
  (set `self.CanFire` true))

(event `self.ReceiveTick`
  (params (DeltaSeconds :type "Float (single-precision)"))
  (if (< (`self.GetDistanceTo` (`GameplayStatics.GetPlayerCharacter` 0)) 2000.0)
    (if (`self.CanFire`)
      (`self.FireMissile`))))

(event `/Game/Variant_Combat/Blueprints/BPI_Damageable.Apply Damage`
  (params (Damage :type "Float (double-precision)") (`Damage Causer` :type "Actor Object Reference") (`Damage Location` :type "Vector Structure") (`Damage Impulse` :type "Vector Structure"))
  (bind _output_get (set `self.Health` (- (`self.Health`) Damage)))
  (if (== _output_get 0.0)
    (`/Game/Variant_Combat/Blueprints/BPI_Damageable.Handle Death`)))

(event `/Game/Variant_Combat/Blueprints/BPI_Damageable.Handle Death`
  (`self.K2_DestroyActor`)
  (bind _returnvalue (`|CreateWidget` "/Game/ProjectSkyjet/UI/WB_LevelComplete.WB_LevelComplete_C"))
  (`UserWidget.AddToViewport` _returnvalue 0))

(fn `FireMissile`
  (bind _arrow (`self.Arrow`))
  (bind _arrow1 (`self.Arrow1`))
  (if (`KismetMathLibrary.RandomBool`)
    (`|SpawnActorFromClass` "/Game/VigilanteContent/Projectiles/West_Missile_AGM114/BP_West_Missile_AGM114.BP_West_Missile_AGM114_C" (`KismetMathLibrary.MakeTransform` (`SceneComponent.K2_GetComponentLocation` _arrow) (`SceneComponent.K2_GetComponentRotation` _arrow)) "Undefined" "MultiplyWithRoot" null null)
    (else
      (`|SpawnActorFromClass` "/Game/VigilanteContent/Projectiles/West_Missile_AGM114/BP_West_Missile_AGM114.BP_West_Missile_AGM114_C" (`KismetMathLibrary.MakeTransform` (`SceneComponent.K2_GetComponentLocation` _arrow1) (`SceneComponent.K2_GetComponentRotation` _arrow1)) "Undefined" "MultiplyWithRoot" null null)))
  (set `self.CanFire` false)
  (`KismetSystemLibrary.K2_SetTimer` null "ResetFire" 0.5))

(fn `ResetFire`
  (set `self.CanFire` true))

(fn `UserConstructionScript`)