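; BP_DroneProjectile is a short-lived drone projectile that damages and knocks back combat characters on hit.
; On spawn, its box ignores its owner and the drone projectiles in the level while moving, and a one-second lifespan starts.
; A hit fires the impact call, sends BP_CombatCharacter targets damage with an impulse built from the impact normal plus upward launch, then destroys the projectile.
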(event `self.Box.OnComponentBeginOverlap`
  (params (OverlappedComponent :type "PrimitiveComponent Object Reference") (OtherActor :type "Actor Object Reference") (OtherComp :type "PrimitiveComponent Object Reference") (OtherBodyIndex :type Integer) (bFromSweep :type Boolean) (SweepResult :type "HitResult Structure (by ref)")))

(event `self.ReceiveBeginPlay`
  (`PrimitiveComponent.IgnoreActorWhenMoving` (`self.Box`) (`self.GetOwner`) true)
  (bind _outactors (`GameplayStatics.GetAllActorsOfClass` "BP_DroneProjectile_C"))
  (for _array_element _outactors
    (`PrimitiveComponent.IgnoreActorWhenMoving` (`self.Box`) _array_element true))
  (`self.SetLifeSpan` 1.0))

(event `self.ReceiveTick`
  (params (DeltaSeconds :type "Float (single-precision)")))

(event `self.Box.OnComponentHit`
  (params (HitComponent :type "PrimitiveComponent Object Reference") (OtherActor :type "Actor Object Reference") (OtherComp :type "PrimitiveComponent Object Reference") (NormalImpulse :type "Vector Structure") (Hit :type "HitResult Structure (by ref)"))
  (bind (_bblockinghit _binitialoverlap _time _distance _location _impactpoint _normal _impactnormal) (`GameplayStatics.BreakHitResult` Hit))
  (`self.OnProjectileImpact` OtherActor Hit)
  (bind _asbp_combat_character (cast `/Game/Variant_Combat/Blueprints/BP_CombatCharacter` OtherActor)
    (:`then`
      (message `/Game/Variant_Combat/Blueprints/BPI_Damageable.Apply Damage` _asbp_combat_character 0.5 null _impactpoint (+ (* _impactnormal (* (`self.Melee Knockback Impulse`) -1.0)) (* (`KismetMathLibrary.Vector_Up`) (`self.Melee Launch Impulse`))))
      (`self.K2_DestroyActor`))
    (:`CastFailed`
      (`self.K2_DestroyActor`))))

(fn `UserConstructionScript`)